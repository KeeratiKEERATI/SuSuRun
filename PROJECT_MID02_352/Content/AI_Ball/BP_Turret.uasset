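; BP_Turret is an AI turret that tracks and shoots at the third-person player character.
; When PawnSensing sees the character, the actor turns in yaw and the Bast component takes interpolated yaw and clamped pitch toward it.
; Each sighting also restarts a short retriggerable delay, which spawns a BP_BULL at BulletSpawn on completion.
; A Collision overlap by the character snaps the actor's pitch and yaw straight at them.
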(event OnSeePawn(PawnSensing)
  (params (Pawn :type Pawn%20Object%20Reference))
  (bind _asbp_third_person_character (Utilities|Casting|CastToBP_ThirdPersonCharacter Pawn))
  (Utilities|FlowControl|Sequence
    (:then_0
      (Transformation|SetWorldRotation (Variables|Default|GetBast) (Math|Rotator|MakeRotator 0.0 (Math|Float|Clamp(Float) (.pitch (Math|Interpolation|RInterpTo (Transformation|GetActorRotation) (Math|Rotator|FindLookatRotation (Transformation|GetActorLocation) (Transformation|GetActorLocation _asbp_third_person_character)) (Utilities|Time|GetWorldDeltaSeconds) (* 2e+01 5.0))) -2e+01 2e+01) (.yaw (Math|Interpolation|RInterpTo (Transformation|GetActorRotation) (Math|Rotator|FindLookatRotation (Transformation|GetActorLocation) (Transformation|GetActorLocation _asbp_third_person_character)) (Utilities|Time|GetWorldDeltaSeconds) (* 2e+01 5.0)))) false false)
      (Transformation|SetActorRotation (Math|Rotator|MakeRotator 0.0 0.0 (.yaw (Math|Interpolation|RInterpTo (Transformation|GetActorRotation) (Math|Rotator|FindLookatRotation (Transformation|GetActorLocation) (Transformation|GetActorLocation _asbp_third_person_character)) (Utilities|Time|GetWorldDeltaSeconds) (* 2e+01 5.0))))))
    (:then_1
      (Utilities|FlowControl|RetriggerableDelay 0.09)
      (Game|SpawnActorfromClass "/Game/AI_Ball/BP_BULL.BP_BULL_C" (Transformation|GetWorldTransform (Variables|Default|GetBullet_spawn)) "Undefined" "MultiplyWithRoot" 0 0))))

(event OnComponentBeginOverlap(Collision)
  (params (OverlappedComponent :type Primitive%20Component%20Object%20Reference) (OtherActor :type Actor%20Object%20Reference) (OtherComp :type Primitive%20Component%20Object%20Reference) (OtherBodyIndex :type Integer) (bFromSweep :type Boolean) (SweepResult :type Hit%20Result%20Structure%20%28by%20ref%29))
  (bind _asbp_third_person_character (Utilities|Casting|CastToBP_ThirdPersonCharacter OtherActor))
  (Transformation|SetActorRotation (Math|Rotator|MakeRotator 0.0 (.pitch (Math|Rotator|FindLookatRotation (Transformation|GetActorLocation) (Transformation|GetActorLocation _asbp_third_person_character))) (.yaw (Math|Rotator|FindLookatRotation (Transformation|GetActorLocation) (Transformation|GetActorLocation _asbp_third_person_character))))))

(fn ConstructionScript)