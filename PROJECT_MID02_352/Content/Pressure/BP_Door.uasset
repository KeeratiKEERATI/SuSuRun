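; BP_Door is a door that moves vertically when enough pressure switches are active.
; SwitchActivated and SwitchDesctivated events raise or lower an active-switch count, then compare it to the required number.
; Meeting the threshold plays the DoorActivation timeline, which drives the Door component's relative Z position, while falling short reverses it.
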(event Custom|SwitchActivated
  (Math|Integer|IncrementInt (Variables|Default|GetPressureSwitchesActive)
    (:%20%20
      (if (>= (Variables|Default|GetPressureSwitchesActive) (Variables|Default|GetPressureSwitchesNeed))
        (bind _doorpotition (Timeline|DoorActivation Play)
          (:Update
            (Transformation|SetRelativeLocation (Variables|Default|GetDoor) (Math|Vector|MakeVector 0.0 0.0 _doorpotition) false false)))
        (else
          (Timeline|DoorActivation Reverse))))))

(event Custom|SwitchDesctivated
  (Math|Integer|DecrementInt (Variables|Default|GetPressureSwitchesActive)
    (:%20%20
      (if (>= (Variables|Default|GetPressureSwitchesActive) (Variables|Default|GetPressureSwitchesNeed))
        (bind _doorpotition (Timeline|DoorActivation Play)
          (:Update
            (Transformation|SetRelativeLocation (Variables|Default|GetDoor) (Math|Vector|MakeVector 0.0 0.0 _doorpotition) false false)))
        (else
          (Timeline|DoorActivation Reverse))))))

(fn ConstructionScript)