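; Boss character that attacks on demand, takes damage and shows its health on a screen widget updated every Tick.
; Attack plays a montage whose notify fires a forward sphere trace from Arrow1 to damage a hit pawn and triggers a world camera shake.
; IsAttack and IsDie gate attacks, though IsDie is never set here.
; At zero health it stops movement, plays a death montage and destroys itself after a delay.
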(event EventAttack
  (bind _arrow1 (Variables|Default|GetArrow1))
  (bind _returnvalue (Transformation|GetWorldLocation _arrow1))
  ;[1 1 1] Attack!
  (if (and (not (Variables|Default|GetisAttack?)) (not (Variables|Default|GetisDie)))
    (Animation|Montage|PlayMontage (Variables|Character|GetMesh) "/Game/My_Characters/AnimationsS/Attack_Modle_Montage.Attack_Modle_Montage"
      (:then
        (Variables|Default|SetisAttack? true))
      (:OnCompleted
        (Variables|Default|SetisAttack? false))
      (:OnNotifyBegin
        (Utilities|FlowControl|Sequence
          (:then_0
            (bind (_outhit _returnvalue_2) (Collision|SphereTraceForObjects _returnvalue (+ _returnvalue (* (Math|Vector|GetForwardVector (Transformation|GetWorldRotation _arrow1)) 3e+03)) 35.0 (Utilities|Array|MakeArray "ObjectTypeQuery3") false 0 "None"))
            (if _returnvalue_2
              (Game|Damage|ApplyDamage (.HitActor (Collision|BreakHitResult _outhit)) 1e+01 0 0)))
          (:then_1
            (Camera|PlayWorldCameraShake "/Game/BOSS_SUSURUN/BP_Sk.BP_Sk_C" (Transformation|GetActorLocation) 0.0 3.5e+03)))))))

(event EventBeginPlay
  (bind _returnvalue (Game|ConstructObjectfromClass "/Game/BOSS_SUSURUN/WB_BossHealth.WB_BossHealth_C"))
  (UserInterface|Viewport|AddtoViewport _returnvalue 0)
  (Variables|Default|SetHealth%20UI _returnvalue))

(event EventTick
  (params (DeltaSeconds :type Float%20%28single-precision%29))
  (Progress|SetPercent (Variables|/Game/BOSS_SUSURUN/WB_BossHealth.WB_BossHealth_C|GetHealthBar (Variables|Default|GetHealth%20UI)) (/ (Variables|Default|GetHealth) 1e+02)))

(event Game|Damage|EventAnyDamage
  (params (Damage :type Float%20%28single-precision%29) (DamageType :type Damage%20Type%20Object%20Reference) (InstigatedBy :type Controller%20Object%20Reference) (DamageCauser :type Actor%20Object%20Reference))
  ;[1 1 1] Health
  (Variables|Default|SetHealth (- (Variables|Default|GetHealth) Damage))
  (if (<= (Variables|Default|GetHealth) 0.0)
    (Pawn|Components|CharacterMovement|DisableMovement (Variables|Character|GetCharacterMovement))
    (Animation|Montage|PlayMontage (Variables|Character|GetMesh) "/Game/My_Characters/AnimationsS/Death_Modle_Montage.Death_Modle_Montage"
      (:then
        (Utilities|FlowControl|Delay 3.0)
        (Actor|DestroyActor)))))

(fn ConstructionScript)